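; BP_Slider is a grabbable slider that moves its static mesh along a straight track, likely for VR motion controllers.
; GrabComponent events store the grabbing controller and clear it when that controller drops.
; While held, Tick snaps the mesh to the controller's closest point on the segment between the spline's first two points.
; IsClosed is true near the second point; material changes are unwired.
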(event OnGrabbed(GrabComponent)
  (params (MotionControler :type Motion%20Controller%20Component%20Object%20Reference))
  (Variables|Default|SetMotion%20Controler%20Ref MotionControler))

(event OnDropped(GrabComponent)
  (params (MotionControler :type Motion%20Controller%20Component%20Object%20Reference))
  (if (== MotionControler (Variables|Default|GetMotion%20Controler%20Ref))
    (Variables|Default|SetMotion%20Controler%20Ref 0)))

(event EventTick
  (params (DeltaSeconds :type Float%20%28single-precision%29))
  (bind _spline (Variables|Default|GetSpline))
  (bind _returnvalue (Spline|GetLocationatSplinePoint _spline 1 "World"))
  (bind _motion_controler_ref (Variables|Default|GetMotion%20Controler%20Ref)
    (:then
      (Transformation|SetWorldLocation (Variables|Default|GetStaticMesh) (Math|Vector|FindClosestPointonSegment (Transformation|GetWorldLocation _motion_controler_ref) (Spline|GetLocationatSplinePoint _spline 0 "World") _returnvalue) false false)
      (if (<= (Math|Vector|VectorLength (- (Math|Vector|FindClosestPointonSegment (Transformation|GetWorldLocation _motion_controler_ref) (Spline|GetLocationatSplinePoint _spline 0 "World") _returnvalue) _returnvalue)) 1e+01)
        (if (not (Variables|Default|GetIs%20Closed))
          (Variables|Default|SetIs%20Closed true))
        (else
          (Variables|Default|SetIs%20Closed false))))
    (:else)))

(fn ConstructionScript)