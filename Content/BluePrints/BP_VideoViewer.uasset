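; BP_VideoViewer plays segments of a video in step with the quest objectives of BP_GameMode.
; It opens the media source on BeginPlay and binds to the game mode's quest updates.
; A "Video" objective seeks the MediaPlayer to that objective's start time and plays.
; Tick polls playback time, pauses at the end time and registers the objective, while a separate StopPlay event toggles play and pause.
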(event Custom|CustomEvent
  (params (ObjectiveID :type Name))
  (bind _mediaplayer (Variables|Default|GetMediaPlayer))
  (if (== ObjectiveID "Video")
    (bind _objective (Default|GetCurentObjective (Variables|Default|GetGameModeRef)))
    (Media|MediaPlayer|Seek _mediaplayer (.starttime _objective))
    (Variables|Default|SetObjective%20End%20Time (.endtime _objective))
    (Media|MediaPlayer|Play _mediaplayer :!class /Script/MediaAssets.MediaPlayer)
    (Variables|Default|SetIsPlaying true)))

(event Custom|StopPlay
  (params (bPlay :type Boolean))
  (bind _mediaplayer (Variables|Default|GetMediaPlayer))
  (if bPlay
    (Media|MediaPlayer|Play _mediaplayer :!class /Script/MediaAssets.MediaPlayer)
    (else
      (Sequencer|Player|Pause _mediaplayer))))

(event EventBeginPlay
  (Class|MediaPlayer|OpenSourceLatent (Variables|Default|GetMediaPlayer) "/Game/Movies/Video_tmp.Video_tmp" (Utilities|Struct|MakeMediaPlayerOptions "(Audio=0,Caption=-1,Metadata=-1,Script=-1,Subtitle=-1,Text=-1,Video=0)" "+00000000.00:00:00.000000000" "UseMediaPlayerSetting" "UseMediaPlayerSetting"))
  (bind _asbp_game_mode (Utilities|Casting|CastToBP_GameMode (Game|GetGameMode)))
  (bind _output_get (Variables|Default|SetGameModeRef _asbp_game_mode))
  (EventDispatchers|BindEventtoQuestUpdate _output_get (delegate Custom|CustomEvent)))

(event EventTick
  (params (DeltaSeconds :type Float%20%28single-precision%29))
  (if (Variables|Default|GetIsPlaying)
    (if (>= (Class|MediaPlayer|GetTime (Variables|Default|GetMediaPlayer)) (Variables|Default|GetObjective%20End%20Time))
      (Sequencer|Player|Pause (Variables|Default|GetMediaPlayer))
      (Variables|Default|SetIsPlaying false)
      (Default|RegisterObjectve (Variables|Default|GetGameModeRef) "Video"))))

(fn ConstructionScript)