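; BP_Array is an actor with an InstancedStaticMesh and a FindClosestTransform function meant to find the instance nearest a given Actor.
; The function loops over the instance count, keeping the smallest distance in ClosestDistance and its loop index in ClosestIndex.
; Each pass reads instance 0's world transform instead of the loop index, and ClosestDistance is not reset within the function.
; The event graph and construction script are empty.
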(event EventBeginPlay)

(event Collision|EventActorBeginOverlap
  (params (OtherActor :type Actor%20Object%20Reference)))

(event EventTick
  (params (DeltaSeconds :type Float%20%28single-precision%29)))

(fn ConstructionScript)

(fn FindClosestTransform
  (params (Actor :type Actor%20Object%20Reference))
  (bind _returnvalue (Transformation|GetActorLocation Actor))
  (bind _instancedstaticmesh (Variables|Default|GetInstancedStaticMesh))
  (bind _outinstancetransform (Components|InstancedStaticMesh|GetInstanceTransform _instancedstaticmesh 0 true))
  (bind _returnvalue_2 (Math|Vector|Distance(Vector) _returnvalue (.location _outinstancetransform)))
  (for _index (range 0 (- (Components|InstancedStaticMesh|GetInstanceCount _instancedstaticmesh) 1))
    (if (< _returnvalue_2 (LocalVariables|GetClosestDistance))
      (LocalVariables|SetClosestDistance _returnvalue_2)
      (LocalVariables|SetClosestIndex _index))))