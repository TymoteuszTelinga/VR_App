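; Game mode that tracks progress through a recipe's ordered list of objectives and quits the game when the recipe is finished.
; On BeginPlay it loads the bread recipe row from a data table into the objective list.
; RegisterObjectve counts matching IDs for the current objective only, advancing once the required count is reached.
; GetCurentObjective returns the active objective.
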(event Custom|RegisterObjectve
  (params (ObjectiveID :type Name))
  (bind _objectislist (Variables|Default|GetObjectisList))
  (bind _curentobjective (Variables|Default|GetCurentObjective))
  (bind _output (Utilities|Array|Get(acopy) _objectislist _curentobjective))
  (if (== ObjectiveID (.objectiveid _output))
    (bind _result (Math|Integer|IncrementInt (Variables|Default|GetObjectiveCount))
      (:%20%20
        (if (>= _result (.count _output))
          (Variables|Default|SetObjectiveCount 0)
          (bind _result_2 (Math|Integer|IncrementInt (Variables|Default|GetCurentObjective))
            (:%20%20
              (if (>= _result_2 (Utilities|Array|Length (Variables|Default|GetObjectisList)))
                (Development|PrintString "Recepi Complited")
                (Game|QuitGame 0 "Quit" false)))))))))

(event EventBeginPlay
  (bind _returnvalue (Utilities|GetDataTableRow (Variables|Default|GetRecepisList) "BreadRecepi")
    (:then
      (bind _output_get (Variables|Default|SetRecepi _returnvalue))
      (Variables|Default|SetObjectisList (.objectives _output_get)))))

(event EventTick
  (params (DeltaSeconds :type Float%20%28single-precision%29)))

(fn ConstructionScript)

(fn GetCurentObjective
  (return (Utilities|Array|Get(acopy) (Variables|Default|GetObjectisList) (Variables|Default|GetCurentObjective))))