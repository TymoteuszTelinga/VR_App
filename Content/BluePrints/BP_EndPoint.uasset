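; BP_EndPoint is the bread delivery point that grades a loaf when it is attached and shows its quality out of 10.
; ScoreBread multiplies factors for form count, cuts, grow rate and bake rate.
; The product is remapped onto the text display, which resets to "Quality" after a short delay.
; The bread is then destroyed, the point freed, and the "Return" objective registered with BP_GameMode.
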(event EventBeginPlay
  (|CallParentFunction)
  (bind _asbp_game_mode (Utilities|Casting|CastToBP_GameMode (Game|GetGameMode)))
  (Variables|Default|SetGasmeModeRef _asbp_game_mode))

(event Collision|EventActorBeginOverlap
  (params (OtherActor :type Actor%20Object%20Reference))
  (|CallParentFunction OtherActor) ; This node is disabled and will not be called.\nDrag off pins to build functionality.
)

(event EventTick
  (params (DeltaSeconds :type Float%20%28single-precision%29))
  (|CallParentFunction DeltaSeconds) ; This node is disabled and will not be called.\nDrag off pins to build functionality.
)

(event EventAttach
  (params (Actor :type BP%20Snappable%20Object%20Reference))
  (|CallParentFunction Actor)
  (bind _asbp_bread_ (Utilities|Casting|CastToBP_Bread_ (Variables|Default|GetActorRef)))
  (bind _finalscore (CallFunction|ScoreBread _asbp_bread_))
  (Rendering|Components|TextRender|SetText (Variables|Default|GetText) (Utilities|Text|FormatText "{score} / 10" (Utilities|Text|ToText(Float) (Math|Float|MapRangeClamped _finalscore 0.0 1.0 0.0 1e+01) "HalfToEven" false true 1 2 0 1)))
  (Utilities|FlowControl|Delay 1.0)
  (Rendering|Components|TextRender|SetText (Variables|Default|GetText) (Utilities|Text|MakeLiteralText "Quality"))
  (Actor|DestroyActor (Variables|Default|GetActorRef))
  (Variables|Default|SetActorRef 0)
  (Variables|Default|SetInUse false)
  (Default|RegisterObjectve (Variables|Default|GetGasmeModeRef) "Return"))

(fn ConstructionScript
  (|CallParentFunction))

(fn ScoreBread
  (params (Bread :type BP%20Bread%20Object%20Reference))
  (LocalVariables|SetScore (* (LocalVariables|GetScore) (Utilities|Select :Index (Variables|/Game/BluePrints/BP_Bread_.BP_Bread__C|GetFormCount Bread) :Option%200 0.2 :Option%201 0.6 :Option%202 0.8 :Option%203 0.9 :Option%204 1.0)))
  (bind _newparam (Default|CutsNumber Bread))
  (LocalVariables|SetScore (* (LocalVariables|GetScore) (Utilities|Select :Index _newparam :Option%200 0.6 :Option%201 0.8 :Option%202 0.9 :Option%203 0.95 :Option%204 1.0)))
  (bind _rate (Default|GrowRate Bread))
  (LocalVariables|SetScore (* _rate (LocalVariables|GetScore)))
  (bind _rate_2 (Default|BakeRate Bread))
  (bind _output_get (LocalVariables|SetScore (* _rate_2 (LocalVariables|GetScore))))
  (return _output_get))

(fn +=
  (params (A :type Float%20%28double-precision%29%20%28by%20ref%29) (B :type Float%20%28double-precision%29))
  (|SetBy-RefVar A (+ A B))
  (return A))