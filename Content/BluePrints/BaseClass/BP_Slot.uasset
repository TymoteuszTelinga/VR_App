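; BP_Slot is a base snap point that previews and holds one BP_Snappable actor.
; When a snappable overlaps its Box while free, a Ghost mesh copies that object's mesh and scale with a ghost material, hiding on exit.
; Attach snaps the given actor onto the Ghost, keeping world scale, and marks the slot in use.
; Dettach only frees the slot and reshows the Ghost, leaving physical detachment out.
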(event OnComponentBeginOverlap(Box)
  (params (OverlappedComponent :type Primitive%20Component%20Object%20Reference) (OtherActor :type Actor%20Object%20Reference) (OtherComp :type Primitive%20Component%20Object%20Reference) (OtherBodyIndex :type Integer) (bFromSweep :type Boolean) (SweepResult :type Hit%20Result%20Structure%20%28by%20ref%29))
  (bind _ghost (Variables|Default|GetGhost))
  (bind _asbp_snappable (Utilities|Casting|CastToBP_Snappable OtherActor))
  (if (not (Variables|Default|GetInUse))
    (Components|StaticMesh|SetStaticMesh _ghost (Variables|/Script/Engine.StaticMeshComponent|GetStaticMesh (Actor|GetComponentbyClass _asbp_snappable "/Script/Engine.StaticMeshComponent")))
    (Rendering|SetVisibility _ghost true false)
    (Transformation|SetWorldScale3D _ghost (.scale (Transformation|GetWorldTransform (Actor|GetComponentbyClass _asbp_snappable "/Script/Engine.StaticMeshComponent"))))
    (for _index (range 0 (Rendering|Material|GetNumMaterials _ghost))
      (Rendering|Material|SetMaterial _ghost _index "/Game/Materials/M_ghost.M_ghost"))))

(event OnComponentEndOverlap(Box)
  (params (OverlappedComponent :type Primitive%20Component%20Object%20Reference) (OtherActor :type Actor%20Object%20Reference) (OtherComp :type Primitive%20Component%20Object%20Reference) (OtherBodyIndex :type Integer))
  (if (not (Variables|Default|GetInUse))
    (Rendering|SetVisibility (Variables|Default|GetGhost) false false)))

(event Custom|Attach
  (params (Actor :type BP%20Snappable%20Object%20Reference))
  (if (not (Variables|Default|GetInUse))
    (Variables|Default|SetInUse true)
    (bind _output_get (Variables|Default|SetActorRef Actor))
    (Transformation|AttachComponentToComponent _output_get (Variables|Default|GetGhost) "None" "SnapToTarget" "SnapToTarget" "KeepWorld" true)
    (Rendering|SetVisibility (Variables|Default|GetGhost) false false)))

(event Custom|Dettach
  (params (Actor :type BP%20Snappable%20Object%20Reference))
  (if (or (not (Utilities|IsValid Actor)) (== Actor (Variables|Default|GetActorRef)))
    (Variables|Default|SetInUse false)
    (Variables|Default|SetActorRef 0)
    (Rendering|SetVisibility (Variables|Default|GetGhost) true false)))

(event EventBeginPlay)

(event Collision|EventActorBeginOverlap
  (params (OtherActor :type Actor%20Object%20Reference)))

(event EventTick
  (params (DeltaSeconds :type Float%20%28single-precision%29)))

(fn ConstructionScript)