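; BP_Slot is a snap slot actor that previews and holds one attached actor at its root.
; When free, overlapping its box shows a Ghost copy of the other actor's static mesh, using a ghost material and matching scale, hidden on overlap end.
; Attach marks the slot in use, snaps the actor to the root and hides the ghost.
; Dettach frees the slot for the stored or an invalid actor and re-shows the ghost.
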(event OnComponentBeginOverlap(Box)
  (params (OverlappedComponent :type Primitive%20Component%20Object%20Reference) (OtherActor :type Actor%20Object%20Reference) (OtherComp :type Primitive%20Component%20Object%20Reference) (OtherBodyIndex :type Integer) (bFromSweep :type Boolean) (SweepResult :type Hit%20Result%20Structure%20%28by%20ref%29))
  (bind _returnvalue (Actor|GetComponentbyClass OtherActor "/Script/Engine.StaticMeshComponent"))
  (bind _ghost (Variables|Default|GetGhost))
  (if (not (Variables|Default|GetInUse))
    (Components|StaticMesh|SetStaticMesh _ghost (Variables|/Script/Engine.StaticMeshComponent|GetStaticMesh _returnvalue))
    (Rendering|SetVisibility _ghost true false)
    (Rendering|Material|SetMaterial _ghost 0 "/Game/Materials/M_ghost.M_ghost")
    (Transformation|SetWorldScale3D _ghost (.scale (Transformation|GetWorldTransform _returnvalue)))))

(event OnComponentEndOverlap(Box)
  (params (OverlappedComponent :type Primitive%20Component%20Object%20Reference) (OtherActor :type Actor%20Object%20Reference) (OtherComp :type Primitive%20Component%20Object%20Reference) (OtherBodyIndex :type Integer))
  (if (not (Variables|Default|GetInUse))
    (Rendering|SetVisibility (Variables|Default|GetGhost) false false)))

(event Custom|Attach
  (params (Actor :type Actor%20Object%20Reference))
  (if (not (Variables|Default|GetInUse))
    (Variables|Default|SetInUse true)
    (bind _output_get (Variables|Default|SetActorRef Actor))
    (Transformation|AttachComponentToComponent _output_get (Variables|Default|GetDefaultSceneRoot) "None" "SnapToTarget" "SnapToTarget" "KeepWorld" true)
    (Rendering|SetVisibility (Variables|Default|GetGhost) false false)))

(event Custom|Dettach
  (params (Actor :type Actor%20Object%20Reference))
  (if (or (not (Utilities|IsValid Actor)) (== Actor (Variables|Default|GetActorRef)))
    (Variables|Default|SetInUse false)
    (Variables|Default|SetActorRef 0)
    (Rendering|SetVisibility (Variables|Default|GetGhost) true false)))

(event EventBeginPlay)

(event Collision|EventActorBeginOverlap
  (params (OtherActor :type Actor%20Object%20Reference)))

(event EventTick
  (params (DeltaSeconds :type Float%20%28single-precision%29)))

(fn ConstructionScript)