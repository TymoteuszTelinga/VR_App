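; Bread actor for a baking game that can be grown, formed, baked and cut, reporting each step to BP_GameMode as an objective.
; Tagged hits drive it: a held roll pin swaps staged meshes on a cooldown, and a knife recolors the material slot matching the nearest spline point.
; Grow and Bake accumulate supplied time through curves into scale and dynamic materials.
; Rate functions score the result, though BakeRate duplicates GrowRate's grow-time formula.
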(event OnComponentBeginOverlap(StaticMesh)
  (params (OverlappedComponent :type Primitive%20Component%20Object%20Reference) (OtherActor :type Actor%20Object%20Reference) (OtherComp :type Primitive%20Component%20Object%20Reference) (OtherBodyIndex :type Integer) (bFromSweep :type Boolean) (SweepResult :type Hit%20Result%20Structure%20%28by%20ref%29))
  (bind _asbp_roll_pin (Utilities|Casting|CastToBP_RollPin OtherActor))
  (if (Variables|/Game/BluePrints/BP_RollPin.BP_RollPin_C|GetIsInHand _asbp_roll_pin)
    (Variables|Default|SetStartOverlap (Transformation|GetActorLocation OtherActor))
    (Development|PrintString "Colision start")))

(event OnComponentHit(StaticMesh)
  (params (HitComponent :type Primitive%20Component%20Object%20Reference) (OtherActor :type Actor%20Object%20Reference) (OtherComp :type Primitive%20Component%20Object%20Reference) (NormalImpulse :type Vector :default "0, 0, 0") (Hit :type Hit%20Result%20Structure%20%28by%20ref%29))
  (bind (_is_valid _output) (CallFunction|ChekTags OtherActor))
  (if _is_valid
    (switch name _output
      (:RollPin
        (CallFunction|Roll OtherActor))
      (:Knife
        (CallFunction|Cut OtherActor Hit)))))

(event OnComponentEndOverlap(StaticMesh)
  (params (OverlappedComponent :type Primitive%20Component%20Object%20Reference) (OtherActor :type Actor%20Object%20Reference) (OtherComp :type Primitive%20Component%20Object%20Reference) (OtherBodyIndex :type Integer))
  (bind _returnvalue (Transformation|GetActorLocation OtherActor))
  (bind _startoverlap (Variables|Default|GetStartOverlap))
  (bind _returnvalue_2 (- _returnvalue _startoverlap))
  (bind _returnvalue_3 (Math|Vector|VectorLength _returnvalue_2))
  (bind _asbp_roll_pin (Utilities|Casting|CastToBP_RollPin OtherActor))
  (if (Variables|/Game/BluePrints/BP_RollPin.BP_RollPin_C|GetIsInHand _asbp_roll_pin)
    (Development|PrintString (Utilities|String|ToString(Float) _returnvalue_3))
    (if (>= _returnvalue_3 1e+01)
      _)))

(event EventBeginPlay
  (bind _asbp_game_mode (Utilities|Casting|CastToBP_GameMode (Game|GetGameMode)))
  (Variables|Default|SetGameModeRef _asbp_game_mode))

(event Collision|EventActorBeginOverlap
  (params (OtherActor :type Actor%20Object%20Reference))
  (|CallParentFunction OtherActor) ; This node is disabled and will not be called.\nDrag off pins to build functionality.
)

(event EventTick
  (params (DeltaSeconds :type Float%20%28single-precision%29))
  (|CallParentFunction DeltaSeconds))

(fn ConstructionScript
  (|CallParentFunction)
  (Utilities|FlowControl|Sequence
    (:then_0
      (bind _returnvalue (Rendering|Material|CreateDynamicMaterialInstance (Variables|Default|GetStaticMesh) 0 "/Game/Materials/M_Bread_Inst.M_Bread_Inst" "None" :!class /Script/Engine.PrimitiveComponent))
      (bind _output_get (Variables|Default|SetMatRef _returnvalue))
      (Rendering|Material|SetScalarParameterValue _output_get "Value" 0.0 :!class /Script/Engine.MaterialInstanceDynamic)
      (Variables|Constants|SetBaseScale (Variables|/Script/Engine.SceneComponent|GetRelativeScale3D (Variables|Default|GetStaticMesh))))
    (:then_1
      (bind _returnvalue_2 (Rendering|Material|CreateDynamicMaterialInstance "/Game/Materials/M_Bread_Inst.M_Bread_Inst" "None" "None" :!class /Script/Engine.KismetMaterialLibrary))
      (bind _output_get_2 (Variables|Default|SetCutMatRef _returnvalue_2))
      (Rendering|Material|SetScalarParameterValue _output_get_2 "Value" 0.1 :!class /Script/Engine.MaterialInstanceDynamic))))

(fn Bake
  (params (Time :type Float%20%28double-precision%29))
  (bind _output_get (Variables|Default|SetDeltaBakeTime (+ Time (Variables|Default|GetDeltaBakeTime))))
  (bind _output_get_2 (Variables|Default|SetIsBaked (> (/ _output_get (Variables|Constants|GetBakeTime)) (Variables|Constants|GetBakeThreshold))))
  (if _output_get_2
    (Default|RegisterObjectve (Variables|Default|GetGameModeRef) "Bake"))
  (Rendering|Material|SetScalarParameterValue (Variables|Default|GetMatRef) "Value" (Math|Curves|GetFloatValue (Variables|Default|GetValueOverTime) (/ _output_get (Variables|Constants|GetBakeTime))) :!class /Script/Engine.MaterialInstanceDynamic)
  (Rendering|Material|SetScalarParameterValue (Variables|Default|GetCutMatRef) "Value" (- (Math|Curves|GetFloatValue (Variables|Default|GetValueOverTime) (/ _output_get (Variables|Constants|GetBakeTime))) 0.1) :!class /Script/Engine.MaterialInstanceDynamic))

(fn Grow
  (params (InTime :type Float%20%28single-precision%29))
  (if (not (Variables|Default|GetIsBaked))
    (bind _output_get (Variables|Default|SetDeltaGrowTime (+ InTime (Variables|Default|GetDeltaGrowTime))))
    (Transformation|SetWorldScale3D (Variables|Default|GetStaticMesh) (+ (Math|Curves|GetVectorValue (Variables|Default|GetSclaeOverTime) (/ _output_get (Variables|Constants|GetGrowTime))) (Variables|Constants|GetBaseScale)))
    (if (> (Variables|Default|GetDeltaGrowTime) (Variables|Constants|GetGrowTime))
      (Default|RegisterObjectve (Variables|Default|GetGameModeRef) "Grow"))))

(fn GrowRate
  (return (- 1.0 (Math|Float|Clamp(Float) (/ (Math|Float|Power (Math|Float|Absolute(Float) (- (Variables|Constants|GetGrowTime) (Variables|Default|GetDeltaGrowTime))) 2.0) (Math|Float|Power (Variables|Constants|GetGrowTime) 2.0)) 0.0 0.8))))

(fn BakeRate
  (return (- 1.0 (Math|Float|Clamp(Float) (/ (Math|Float|Power (Math|Float|Absolute(Float) (- (Variables|Constants|GetGrowTime) (Variables|Default|GetDeltaGrowTime))) 2.0) (Math|Float|Power (Variables|Constants|GetGrowTime) 2.0)) 0.0 0.8))))

(fn Roll
  (params (Object :type Object%20Object%20Reference))
  (bind _staticmesh (Variables|Default|GetStaticMesh))
  (bind _asbp_roll_pin (Utilities|Casting|CastToBP_RollPin Object))
  (if (Variables|Default|GetCan%20Be%20Formed)
    (if (Variables|/Game/BluePrints/BP_RollPin.BP_RollPin_C|GetIsInHand _asbp_roll_pin)
      (if (and (not (Variables|Default|GetIsBaked)) (> (Utilities|Array|Length (Variables|Constants|GetModelsSteps)) (Variables|Default|GetFormCount)))
        (Components|StaticMesh|SetStaticMesh (Variables|Default|GetStaticMesh) (Utilities|Array|Get(acopy) (Variables|Constants|GetModelsSteps) (Variables|Default|GetFormCount)))
        (for _index (range 0 (Rendering|Material|GetNumMaterials _staticmesh))
          (Rendering|Material|SetMaterial _staticmesh _index (Variables|Default|GetMatRef))
          (Default|RegisterObjectve (Variables|Default|GetGameModeRef) "Form"))
        (Math|Integer|IncrementInt (Variables|Default|GetFormCount)
          (:%20%20
            (Variables|Default|SetCan%20Be%20Formed false)
            (Utilities|Time|SetTimerbyFunctionName 0 "ResetCooldown" 0.1)))))))

(fn Cut
  (params (Object :type Object%20Object%20Reference) (Hit :type Hit%20Result%20Structure%20%28by%20ref%29))
  (bind _spline (Variables|Default|GetSpline))
  (Utilities|Casting|CastToBP_Knife Object)
  (LocalVariables|SetClosest%20Distans 1.2e+02)
  (LocalVariables|Setclosest%20Point 0)
  (for _index (range 0 (- (Spline|GetNumberOfSplinePoints _spline) 1))
    (if (< (Math|Vector|VectorLength (- (Spline|GetLocationatSplinePoint _spline _index "World") (.ImpactPoint (Collision|BreakHitResult Hit)))) (LocalVariables|GetClosest%20Distans))
      (LocalVariables|SetClosest%20Distans (Math|Vector|VectorLength (- (Spline|GetLocationatSplinePoint _spline _index "World") (.ImpactPoint (Collision|BreakHitResult Hit)))))
      (LocalVariables|Setclosest%20Point _index)))
  (if (not (>= (LocalVariables|GetClosest%20Distans) 1e+02))
    (Rendering|Material|SetMaterial (Variables|Default|GetStaticMesh) (+ (LocalVariables|Getclosest%20Point) 1) (Variables|Default|GetCutMatRef))
    (Default|RegisterObjectve (Variables|Default|GetGameModeRef) "Cut")
    (Utilities|Array|SetArrayElem (Variables|Default|GetUniqueCuts) (LocalVariables|Getclosest%20Point) true)))

(fn ChekTags
  (params (self2 :type Actor%20Object%20Reference))
  (bind _tags (Variables|/Script/Engine.Actor|GetTags self2))
  (if (> (Utilities|Array|Length _tags) 0)
    (return true (Utilities|Array|Get(acopy) _tags))
    (else
      (return false "None"))))

(fn CutsNumber
  (for _array_element (Variables|Default|GetUniqueCuts)
    (if _array_element
      (Math|Integer|IncrementInt (LocalVariables|GetCutsNumber))))
  (return (LocalVariables|GetCutsNumber)))

(fn ResetCooldown
  (Variables|Default|SetCan%20Be%20Formed true))