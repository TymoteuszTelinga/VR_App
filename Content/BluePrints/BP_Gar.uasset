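; BP_Gar is a dough container that dispenses a limited supply of BP_Bread_ actors, starting from RefilCount.
; It spawns one owned bread at its Collider; when that leaves, it releases ownership, spawns the next and reports the "GetDough" objective to BP_GameMode.
; The Filing component's Z scale shrinks with the remaining count.
; A leftover IA_Shoot_Right handler spawns bread without the count check; its input-context setup is disconnected.
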(event OnComponentBeginOverlap(Collider)
  (params (OverlappedComponent :type Primitive%20Component%20Object%20Reference) (OtherActor :type Actor%20Object%20Reference) (OtherComp :type Primitive%20Component%20Object%20Reference) (OtherBodyIndex :type Integer) (bFromSweep :type Boolean) (SweepResult :type Hit%20Result%20Structure%20%28by%20ref%29))
  ;[1 1 1] Old System
)

(event OnComponentEndOverlap(Collider)
  (params (OverlappedComponent :type Primitive%20Component%20Object%20Reference) (OtherActor :type Actor%20Object%20Reference) (OtherComp :type Primitive%20Component%20Object%20Reference) (OtherBodyIndex :type Integer))
  (if (== (Components|GetOwner OtherActor) self)
    (Actor|SetOwner OtherActor 0)
    (CallFunction|SpawnBread)
    (CallFunction|AdjustFilling)
    (Default|RegisterObjectve (Variables|Default|GetGameModeRef) "GetDough")))

(event OnComponentEndOverlap(Filing)
  (params (OverlappedComponent :type Primitive%20Component%20Object%20Reference) (OtherActor :type Actor%20Object%20Reference) (OtherComp :type Primitive%20Component%20Object%20Reference) (OtherBodyIndex :type Integer)))

(event Input|EnhancedActionEvents|EnhancedInputActionIA_Shoot_Right
  (params (ActionValue :type Boolean) (ElapsedSeconds :type Float%20%28double-precision%29) (TriggeredSeconds :type Float%20%28double-precision%29) (InputAction :type Input%20Action%20Object%20Reference :default "/Game/VRTemplate/Input/Actions/IA_Shoot_Right.IA_Shoot_Right"))
  (bind _collider (Variables|Default|GetCollider))
  (bind _returnvalue (Transformation|GetWorldTransform _collider))
  ;[1 1 1] Old System
  (:Started
    (Game|SpawnActorfromClass "/Game/BluePrints/BP_Bread_.BP_Bread__C" (Math|Transform|MakeTransform (.location _returnvalue) (.rotation _returnvalue) "1.000000,1.000000,1.000000") "AdjustIfPossibleButAlwaysSpawn" 0 0)
    (Development|PrintString "Spawned bread")))

(event EventBeginPlay
  (Variables|Default|SetCount (Variables|Default|GetRefilCount))
  (CallFunction|SpawnBread)
  (bind _asbp_game_mode (Utilities|Casting|CastToBP_GameMode (Game|GetGameMode)))
  (Variables|Default|SetGameModeRef _asbp_game_mode))

(event Collision|EventActorBeginOverlap
  (params (OtherActor :type Actor%20Object%20Reference)))

(event EventTick
  (params (DeltaSeconds :type Float%20%28single-precision%29)))

(fn ConstructionScript
  (bind _returnvalue (Rendering|Material|CreateDynamicMaterialInstance (Variables|Default|GetFiling) 0 "/Game/Materials/M_Bread_Inst.M_Bread_Inst" "None" :!class /Script/Engine.PrimitiveComponent))
  (Rendering|Material|SetScalarParameterValue _returnvalue "Value" 0.0 :!class /Script/Engine.MaterialInstanceDynamic)
  (Variables|Default|SetBaseFillingScale (Variables|/Script/Engine.SceneComponent|GetRelativeScale3D (Variables|Default|GetFiling))))

(fn SpawnBread
  (bind _collider (Variables|Default|GetCollider))
  (bind _returnvalue (Transformation|GetWorldTransform _collider))
  (if (> (Variables|Default|GetCount) 0)
    (Game|SpawnActorfromClass "/Game/BluePrints/BP_Bread_.BP_Bread__C" (Math|Transform|MakeTransform (.location _returnvalue) (.rotation _returnvalue) "1.000000,1.000000,1.000000") "AlwaysSpawn" self 0)
    (Math|Integer|DecrementInt (Variables|Default|GetCount))))

(fn AdjustFilling
  (bind _basefillingscale (Variables|Default|GetBaseFillingScale))
  (Transformation|SetRelativeScale3D (Variables|Default|GetFiling) (Math|Vector|MakeVector (.x _basefillingscale) (.y _basefillingscale) (Math|Float|Lerp 0.0 (Variables|Default|GetFullScale) (/ (Variables|Default|GetCount) (Variables|Default|GetRefilCount))))))