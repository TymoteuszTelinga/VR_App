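; BP_Lever is a lever whose handle follows the motion controller that grabs it.
; GrabComponent stores the controller reference on grab and clears it when that same controller drops the lever.
; While held, Tick converts the controller's position into the handle's space with a 90-degree offset and adds its look-at pitch to the handle's pitch, clamped between 0 and 90 degrees.
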(event OnGrabbed(GrabComponent)
  (params (MotionControler :type Motion%20Controller%20Component%20Object%20Reference))
  (Variables|Default|SetMotion%20Controler%20Ref MotionControler))

(event OnDropped(GrabComponent)
  (params (MotionControler :type Motion%20Controller%20Component%20Object%20Reference))
  (if (== MotionControler (Variables|Default|GetMotion%20Controler%20Ref))
    (Variables|Default|SetMotion%20Controler%20Ref 0)))

(event EventTick
  (params (DeltaSeconds :type Float%20%28single-precision%29))
  (bind _handle (Variables|Default|GetHandle))
  (bind _handle_2 (Variables|Default|GetHandle))
  (bind _returnvalue (Transformation|GetWorldTransform _handle))
  (bind _relativerotation (Variables|/Script/Engine.SceneComponent|GetRelativeRotation _handle_2))
  (bind _motion_controler_ref (Variables|Default|GetMotion%20Controler%20Ref)
    (:then
      (Transformation|SetRelativeRotation _handle_2 (Math|Rotator|MakeRotator (.roll _relativerotation) (Math|Float|Clamp(Float) (+ (.pitch _relativerotation) (.pitch (Math|Rotator|FindLookatRotation (Math|Vector|MakeVector 0.0 0.0 0.0) (.location (Math|Transform|MakeRelativeTransform (Transformation|GetWorldTransform _motion_controler_ref) (Math|Transform|MakeTransform (.location _returnvalue) (Math|Rotator|CombineRotators (.rotation _returnvalue) "90.000000,0.000000,0.000000") (.scale _returnvalue))))))) 0.0 9e+01) (.yaw _relativerotation)) false false))
    (:else)))

(fn ConstructionScript)