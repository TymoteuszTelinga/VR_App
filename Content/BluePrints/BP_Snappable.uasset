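; BP_Snappable is a grabbable actor that snaps into BP_Slot actors.
; Overlap events store the most recently entered slot in SlorRef and clear it when that same slot's overlap ends.
; GrabComponent events use that reference, asking the slot to attach the actor on drop and detach it on grab.
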(event OnDropped(GrabComponent)
  (Utilities|IsValid (Variables|Default|GetSlorRef)
    (:Is%20Valid
      (Default|Attach (Variables|Default|GetSlorRef) self))))

(event OnGrabbed(GrabComponent)
  (Utilities|IsValid (Variables|Default|GetSlorRef)
    (:Is%20Valid
      (Default|Dettach (Variables|Default|GetSlorRef) self))))

(event Collision|EventActorBeginOverlap
  (params (OtherActor :type Actor%20Object%20Reference))
  (bind _asbp_slot (Utilities|Casting|CastToBP_Slot OtherActor))
  (Variables|Default|SetSlorRef _asbp_slot))

(event EventTick
  (params (DeltaSeconds :type Float%20%28single-precision%29)))

(event Collision|EventActorEndOverlap
  (params (OtherActor :type Actor%20Object%20Reference))
  (bind _asbp_slot (Utilities|Casting|CastToBP_Slot OtherActor))
  (if (== _asbp_slot (Variables|Default|GetSlorRef))
    (Variables|Default|SetSlorRef 0)))

(fn ConstructionScript)